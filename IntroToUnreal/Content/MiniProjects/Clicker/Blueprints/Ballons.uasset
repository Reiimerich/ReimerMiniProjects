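; Balloon actor for a Clicker mini-project that grows until it pops.
; Each IncreaseSize call adds the Increase value to the Sphere's world scale, then checks the scale vector's length against a threshold.
; Past the threshold it spawns an explosion particle and destroys itself; otherwise it pushes the Sphere upward with a mass-independent force.
; The event graph is empty, so nothing in this Blueprint calls IncreaseSize.
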(event EventBeginPlay)

(event Collision|EventActorBeginOverlap
  (params (OtherActor :type Actor%20Object%20Reference)))

(event EventTick
  (params (DeltaSeconds :type Float%20%28single-precision%29)))

(fn ConstructionScript)

(fn IncreaseSize
  (bind _sphere (Variables|Default|GetSphere))
  (bind _returnvalue (Transformation|GetWorldScale _sphere))
  (Transformation|SetWorldScale3D (Variables|Default|GetSphere) (+ _returnvalue (Variables|Default|GetIncrease)))
  (if (> (Math|Vector|VectorLength _returnvalue) 3.0)
    (Effects|SpawnEmitteratLocation "/Game/StarterContent/Particles/P_Explosion.P_Explosion" (Transformation|GetWorldLocation (Variables|Default|GetSphere)))
    (Actor|DestroyActor)
    (else
      (Physics|AddForce (Variables|Default|GetSphere) "0, 0,75000.000000" "None" true))))